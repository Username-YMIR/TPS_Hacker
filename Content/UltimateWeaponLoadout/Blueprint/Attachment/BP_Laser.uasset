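; BP_Laser is a weapon attachment Blueprint that switches a laser beam on and off.
; On enable, ToggleAttachment adds a static mesh component at runtime, snaps it to LaserSocket on the attachment's StaticMesh, stretches it along X and stores it as LaserCurrent.
; On disable, it destroys that stored component.
; The beam is only a scaled mesh, with no trace or per-frame update.
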(event EventBeginPlay
  (|CallParentFunction) ; This node is disabled and will not be called.\nDrag off pins to build functionality.
)

(event Collision|EventActorBeginOverlap
  (params (OtherActor :type Actor%20Object%20Reference))
  (|CallParentFunction OtherActor) ; This node is disabled and will not be called.\nDrag off pins to build functionality.
)

(event EventTick
  (params (DeltaSeconds :type Float%20%28single-precision%29))
  (|CallParentFunction DeltaSeconds) ; This node is disabled and will not be called.\nDrag off pins to build functionality.
)

(event EventToggleAttachment
  (params (Value :type Boolean))
  (if Value
    (bind _returnvalue (AddComponent|AddStaticMeshComponent true))
    (Transformation|AttachComponentToComponent _returnvalue (Variables|Default|GetStaticMesh) "LaserSocket" "SnapToTarget" "SnapToTarget" "SnapToTarget" true)
    (bind _output_get (Variables|Default|SetLaserCurrent _returnvalue))
    (Transformation|SetWorldScale3D _output_get "100.000000,5.000000,5.000000")
    (else
      (Components|DestroyComponent (Variables|Default|GetLaserCurrent)))))

(fn ConstructionScript
  (|CallParentFunction))