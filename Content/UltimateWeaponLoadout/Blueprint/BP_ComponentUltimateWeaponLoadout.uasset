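; Character component that manages the weapon loadout, crosshair and basic weapon actions.
; BeginSettings loads the saved weapons from the GameInstance; EquipWeapon spawns the configured actor on a mesh socket, updates the animation overlay and saves the slot.
; The loadout menu switches the view to a preview actor spawned far off in the world, and RemoveMainLoadout restores it.
; Camera line traces drive interaction and hitscan damage, while a toggle messages weapon attachments.
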(event Custom|BeginSettings
  (params (Camera :type Camera%20Component%20Object%20Reference) (Character :type Character%20Object%20Reference) (OwningPlayer :type Player%20Controller%20Object%20Reference))
  ;[1 1 1] Begin Settings
  (Variables|Default|SetCamera Camera)
  (Variables|Default|SetCharacter Character)
  (Variables|Default|SetOwning%20Player%20Controller OwningPlayer)
  (CallFunction|LoadWeaponSave)
  (bind _returnvalue (UserInterface|CreateWidget "/Game/UltimateWeaponLoadout/Blueprint/Widget/WB_Crosshair.WB_Crosshair_C"))
  (bind _output_get (Variables|Default|SetWBCrosshair _returnvalue))
  (UserInterface|Viewport|AddtoViewport _output_get 0))

(event Custom|Character_Interact
  (bind _camera (Variables|Default|GetCamera))
  (bind _returnvalue (Transformation|GetWorldLocation _camera))
  ;[1 1 1] Interact Weapon
  (bind _outhit (Collision|LineTraceByChannel _returnvalue (+ _returnvalue (* (Math|Vector|GetForwardVector (Transformation|GetWorldRotation _camera)) 5e+02)) "TraceTypeQuery1" false 0 "ForDuration"))
  (Class|BPInterfaceUltimateWeaponLoadout|Interact(Message) (.HitActor (Collision|BreakHitResult _outhit)) self))

(event Custom|Open%20Loadout%20Menu
  (bind _character (Variables|Default|GetCharacter))
  ;[1 1 1] Open Widget loadout
  (if (not (Variables|Default|GetLoadOut%20Open?))
    (Widget|RemovefromParent (Variables|Default|GetWBCrosshair))
    (Variables|Default|SetLoadOut%20Open? true)
    (bind _returnvalue (Game|SpawnActorfromClass :Class "/Game/UltimateWeaponLoadout/Blueprint/Weapon/PreviewWeapon/BP_ShowWeaponSelect.BP_ShowWeaponSelect_C" :SpawnTransform (Math|Transform|MakeTransform "100000.000000,100000.000000,10000.000000" "0, 0, 0" "1.000000,1.000000,1.000000") :CollisionHandlingOverride "Undefined" :TransformScaleMethod "OverrideRootScale" :Owner _character :Character _character :Component self :Instigator _character))
    (Game|Player|SetViewTargetwithBlend (Variables|Default|GetOwning%20Player%20Controller) _returnvalue 0.0 "VTBlend_Linear" 0.0 false)
    (bind _returnvalue_2 (UserInterface|CreateWidget "/Game/UltimateWeaponLoadout/Blueprint/Widget/WB_MainLoadout.WB_MainLoadout_C" (Variables|Default|GetOwning%20Player%20Controller) self _returnvalue))
    (UserInterface|Viewport|AddtoViewport _returnvalue_2 0)))

(event Custom|EventToggleAttachment
  ;[1 1 1] Event Toggle flashlight or laser
  (if (Variables|Default|GetActiveEventAttachment)
    (Variables|Default|SetActiveEventAttachment false)
    (else
      (Variables|Default|SetActiveEventAttachment true)))
  (bind _weapon_current (Variables|Default|GetWeapon%20Current)
    (:then
      (for _array_element (Variables|/Game/UltimateWeaponLoadout/Blueprint/Weapon/BP_Weaponbase.BP_Weaponbase_C|GetActorsAttachment _weapon_current)
        (Class|BPInterfaceUltimateWeaponLoadout|ToggleAttachment(Message) _array_element (Variables|Default|GetActiveEventAttachment))))
    (:else)))

(event Custom|FireWeapon
  (bind _camera (Variables|Default|GetCamera))
  (bind _returnvalue (Transformation|GetWorldLocation _camera))
  ;[1 1 1] Fire Weapon
  (Variables|Default|GetWeapon%20Current
    (:then
      (bind (_outhit _returnvalue_2) (Collision|LineTraceByChannel _returnvalue (+ _returnvalue (* (Math|Vector|GetForwardVector _camera) 1.5e+05)) "TraceTypeQuery1" false 0 "None"))
      (if _returnvalue_2
        (Game|Damage|ApplyPointDamage (.HitActor (Collision|BreakHitResult _outhit)) 1e+01 (.ImpactPoint (Collision|BreakHitResult _outhit)) _outhit)))
    (:else)))

(fn EquipWeapon
  (params (ConfigWeapon :type S%20Weapon%20Config%20Structure) (Slot :type E_TypeSlot%20Enum :default "NewEnumerator2"))
  (bind _character (Variables|Default|GetCharacter))
  (bind (_actor _socket _animationstate) (Utilities|Struct|BreakS_WeaponConfig ConfigWeapon))
  (bind _weapon_current (Variables|Default|GetWeapon%20Current)
    (:then
      (Actor|DestroyActor _weapon_current))
    (:else
      _))
  (bind _returnvalue (Game|SpawnActorfromClass _actor (Math|Transform|MakeTransform "0, 0, 0" "0, 0, 0" "1.000000,1.000000,1.000000") "Undefined" "SelectDefaultAtRuntime" _character ConfigWeapon "None" _character))
  (Variables|Default|SetWeapon%20Current _returnvalue)
  (Transformation|AttachComponentToComponent _returnvalue (Variables|/Script/Engine.Character|GetMesh (Variables|Default|GetCharacter)) _socket "SnapToTarget" "SnapToTarget" "SnapToTarget" true)
  (Default|CallUpdateOverlayAnimation _animationstate)
  (switch Utilities|FlowControl|Switch|SwitchonE_TypeSlot Slot
    (:NewEnumerator2
      (Default|SaveWeaponSlot (Variables|Default|GetGame%20Instance) (Variables|/Game/UltimateWeaponLoadout/Blueprint/Weapon/BP_Weaponbase.BP_Weaponbase_C|GetS_WeaponConfig (Variables|Default|GetWeapon%20Current)) "NewEnumerator2"))
    (:NewEnumerator0
      (bind _output_get (Variables|Default|SetWeapon%20Primary (Variables|Default|GetWeapon%20Current)))
      (bind _output_get_2 (Variables|Default|SetWeapon%20Primary%20Config (Variables|/Game/UltimateWeaponLoadout/Blueprint/Weapon/BP_Weaponbase.BP_Weaponbase_C|GetS_WeaponConfig _output_get)))
      (Default|SaveWeaponSlot (Variables|Default|GetGame%20Instance) _output_get_2 "NewEnumerator0"))
    (:NewEnumerator1
      (bind _output_get_3 (Variables|Default|SetWeapon%20Secondary (Variables|Default|GetWeapon%20Current)))
      (bind _output_get_4 (Variables|Default|SetWeapon%20Secondary%20Config (Variables|/Game/UltimateWeaponLoadout/Blueprint/Weapon/BP_Weaponbase.BP_Weaponbase_C|GetS_WeaponConfig _output_get_3)))
      (Default|SaveWeaponSlot (Variables|Default|GetGame%20Instance) _output_get_4 "NewEnumerator1")
      (return true)))
  (return true))

(fn RemoveMainLoadout
  (bind _outactors (Actor|GetAllActorsOfClass "/Game/UltimateWeaponLoadout/Blueprint/Weapon/PreviewWeapon/BP_ShowWeaponSelect.BP_ShowWeaponSelect_C"))
  (for _array_element _outactors
    (Utilities|IsValid _array_element
      (:Is%20Valid
        (Actor|DestroyActor _array_element))))
  (bind _foundwidgets (Widget|GetAllWidgetsOfClass "/Game/UltimateWeaponLoadout/Blueprint/Widget/WB_MainSelectWeapon.WB_MainSelectWeapon_C" true))
  (for _array_element_2 _foundwidgets
    (Utilities|IsValid _array_element_2
      (:Is%20Valid
        (Widget|RemovefromParent _array_element_2))))
  (bind _owning_player_controller (Variables|Default|GetOwning%20Player%20Controller)
    (:then
      (Game|Player|SetViewTargetwithBlend _owning_player_controller (Variables|Default|GetCharacter) 0.0 "VTBlend_Linear" 0.0 false)
      (Variables|/Script/Engine.PlayerController|SetbShowMouseCursor _owning_player_controller false)
      (Input|SetInputModeGameOnly _owning_player_controller false))
    (:else
      _))
  (Variables|Default|SetLoadOut%20Open? false)
  (UserInterface|Viewport|AddtoViewport (Variables|Default|GetWBCrosshair) 0)
  (return))

(fn LoadWeaponSave
  (bind _asbp_game_instance_fps_weapon_customization (Utilities|Casting|CastToBP_GameInstanceFpsWeaponCustomization (Game|GetGameInstance)))
  (bind _output_get (Variables|Default|SetGame%20Instance _asbp_game_instance_fps_weapon_customization))
  (Variables|Default|SetWeapon%20Current%20Config (Variables|/Game/UltimateWeaponLoadout/Blueprint/SaveGame/BP_SaveFpsWeaponCustomization.BP_SaveFpsWeaponCustomization_C|GetWeapon%20Current (Variables|/Game/UltimateWeaponLoadout/Blueprint/SaveGame/BP_GameInstanceFpsWeaponCustomization.BP_GameInstanceFpsWeaponCustomization_C|GetCurrentSaveGame _output_get)))
  (Variables|Default|SetWeapon%20Primary%20Config (Variables|/Game/UltimateWeaponLoadout/Blueprint/SaveGame/BP_SaveFpsWeaponCustomization.BP_SaveFpsWeaponCustomization_C|GetWeapon%20Primary (Variables|/Game/UltimateWeaponLoadout/Blueprint/SaveGame/BP_GameInstanceFpsWeaponCustomization.BP_GameInstanceFpsWeaponCustomization_C|GetCurrentSaveGame _output_get)))
  (Variables|Default|SetWeapon%20Secondary%20Config (Variables|/Game/UltimateWeaponLoadout/Blueprint/SaveGame/BP_SaveFpsWeaponCustomization.BP_SaveFpsWeaponCustomization_C|GetWeapon%20Secondary (Variables|/Game/UltimateWeaponLoadout/Blueprint/SaveGame/BP_GameInstanceFpsWeaponCustomization.BP_GameInstanceFpsWeaponCustomization_C|GetCurrentSaveGame _output_get)))
  (CallFunction|EquipWeapon (Variables|Default|GetWeapon%20Current%20Config) "NewEnumerator2"))

(fn GetLeftHandSocket
  (params (Character :type Character%20Object%20Reference))
  (return ""))