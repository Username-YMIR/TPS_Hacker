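; Base weapon actor that builds its mesh from a weapon config or DT_Weapons row and acts as an interactable pickup.
; Interact passes the config to the interacting component's EquipWeapon, destroying the actor on success.
; Configured attachments spawn on BeginPlay as socketed actors, one per type, and are cleaned up on destruction.
; GetLeftHandSocket converts the Ik_Hand_L socket into hand_r bone space, keeping left-hand placement relative to the right hand.
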(event Custom|Spawn%20Attachments
  (for _array_element (.AttachmentCurrent (Utilities|Struct|BreakS_WeaponConfig (Variables|Default|GetS_WeaponConfig)))
    (CallFunction|ApplyAttachment _array_element)))

(event EventBeginPlay
  (CallFunction|SpawnAttachments))

(event Collision|EventActorBeginOverlap
  (params (OtherActor :type Actor%20Object%20Reference)))

(event EventInteract
  (params (Component :type BP%20Component%20Ultimate%20Weapon%20Loadout%20Object%20Reference))
  (bind _value (Default|EquipWeapon Component (Variables|Default|GetS_WeaponConfig) "NewEnumerator2"))
  (if _value
    (Actor|DestroyActor)))

(event EventDestroyed
  (CallFunction|RemoveAllAtchmentsActors))

(fn ConstructionScript
  (if (!= (.Name (Utilities|Struct|BreakS_WeaponConfig (Variables|Default|GetS_WeaponConfig))) "")
    (Components|SkeletalMesh|SetSkeletalMeshAsset (Variables|Default|GetSkeletalMesh) (.SkeletalMesh (Utilities|Struct|BreakS_WeaponConfig (Variables|Default|GetS_WeaponConfig))))
    (else
      (bind _returnvalue (Utilities|GetDataTableRow "/Game/UltimateWeaponLoadout/Blueprint/Weapon/DT_Weapons.DT_Weapons" (Variables|Default|GetRow%20Name))
        (:then
          (Variables|Default|SetS_WeaponConfig _returnvalue)
          (Components|SkeletalMesh|SetSkeletalMeshAsset (Variables|Default|GetSkeletalMesh) (.SkeletalMesh (Utilities|Struct|BreakS_WeaponConfig (Variables|Default|GetS_WeaponConfig)))))))))

(fn ApplyAttachment
  (params (Class :type S%20Attachment%20Type%20Structure))
  (bind (_attachmenttype _actorclass _socketspawn) (Utilities|Struct|BreakS_AttachmentType Class))
  (CallFunction|RemoveAttachment Class)
  (bind _returnvalue (Game|SpawnActorfromClass _actorclass (Math|Transform|MakeTransform "0, 0, 0" "0, 0, 0" (.scale (Transformation|GetSocketTransform (Variables|Default|GetSkeletalMesh) _socketspawn "RTS_World"))) "Undefined" "SelectDefaultAtRuntime" 0 Class 0))
  (Transformation|AttachComponentToComponent _returnvalue (Variables|Default|GetSkeletalMesh) _socketspawn "SnapToTarget" "SnapToTarget" "SnapToTarget" true)
  (Utilities|Array|Add (Variables|Default|GetEquipedAttachments) Class)
  (Utilities|Array|Add (Variables|Default|GetActorsAttachment) _returnvalue)
  (Class|BPInterfaceUltimateWeaponLoadout|ToggleAttachment(Message) _returnvalue true))

(fn RemoveAttachment
  (params (Class :type S%20Attachment%20Type%20Structure))
  (for (_array_element _array_index) (Variables|Default|GetEquipedAttachments)
    (if (Utilities|Enum|Equal(Enum) (.AttachmentType (Utilities|Struct|BreakS_AttachmentType Class)) (.AttachmentType (Utilities|Struct|BreakS_AttachmentType _array_element)))
      (Utilities|Array|RemoveIndex (Variables|Default|GetEquipedAttachments) _array_index)
      (Class|BPInterfaceUltimateWeaponLoadout|DestroyAttachment(Message) (Utilities|Array|Get(acopy) (Variables|Default|GetActorsAttachment) _array_index))
      (Utilities|Array|RemoveIndex (Variables|Default|GetActorsAttachment) _array_index))))

(fn RemoveAllAtchmentsActors
  (for _array_element (Variables|Default|GetActorsAttachment)
    (Utilities|IsValid _array_element
      (:Is%20Valid
        (Class|BPInterfaceUltimateWeaponLoadout|DestroyAttachment(Message) _array_element))))
  (Utilities|Array|Clear (Variables|Default|GetActorsAttachment))
  (Utilities|Array|Clear (Variables|Default|GetEquipedAttachments))
  (return))

(fn GetLeftHandSocket
  (params (Character :type Character%20Object%20Reference))
  (return (Math|Transform|MakeTransform (.OutPosition (Class|SkinnedMeshComponent|TransformtoBoneSpace (Variables|/Script/Engine.Character|GetMesh Character) "hand_r" (.location (Transformation|GetSocketTransform (Variables|Default|GetSkeletalMesh) "Ik_Hand_L" "RTS_World")) "0, 0, 0")) "0, 0, 0" "1.000000,1.000000,1.000000")))