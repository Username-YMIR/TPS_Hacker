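; SaveGame object storing the player's FPS weapon loadout: every weapon config with its attachments, plus Current, Primary and Secondary slots.
; CreateSaveWeapon seeds the list from DT_Weapons, defaulting to Rifle as primary and current, Pistol as secondary.
; Attachment add/remove rebuilds the entry from its table row, keeping only the edited attachment list, and returns it.
; CheckSaveSlotWeaapon refreshes only the first slot matching by name, checking Current first.
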(fn CreateSaveWeapon
  (bind _outrownames (DataTable|GetDataTableRowNames "/Game/UltimateWeaponLoadout/Blueprint/Weapon/DT_Weapons.DT_Weapons"))
  (for _array_element _outrownames
    (bind _returnvalue (Utilities|GetDataTableRow "/Game/UltimateWeaponLoadout/Blueprint/Weapon/DT_Weapons.DT_Weapons" _array_element)
      (:then
        (Utilities|Array|Add (Variables|Default|GetWeapons) _returnvalue))))
  (bind _returnvalue_2 (Utilities|GetDataTableRow "/Game/UltimateWeaponLoadout/Blueprint/Weapon/DT_Weapons.DT_Weapons" "Rifle")
    (:then
      (bind _output_get (Variables|Default|SetWeapon%20Primary _returnvalue_2))
      (Variables|Default|SetWeapon%20Current _output_get)
      (bind _returnvalue_3 (Utilities|GetDataTableRow "/Game/UltimateWeaponLoadout/Blueprint/Weapon/DT_Weapons.DT_Weapons" "Pistol")
        (:then
          (Variables|Default|SetWeapon%20Secondary _returnvalue_3))))))

(fn SaveApplyAttachmentWeapon
  (params (Weapon :type S%20Weapon%20Config%20Structure) (Attachment :type S%20Attachment%20Type%20Structure))
  (bind (_array_element _array_index) (Utilities|Array|ForEachLoopwithBreak (Variables|Default|GetWeapons) :!label _label)
    (:LoopBody
      (if (== (.Name (Utilities|Struct|BreakS_WeaponConfig _array_element)) (.Name (Utilities|Struct|BreakS_WeaponConfig Weapon)))
        (LocalVariables|Setlocal%20ID _array_index)
        (LocalVariables|SetLocal%20Attachment (.AttachmentCurrent (Utilities|Struct|BreakS_WeaponConfig (Utilities|Array|Get(acopy) (Variables|Default|GetWeapons) (LocalVariables|Getlocal%20ID)))))
        (Utilities|Array|AddUnique (LocalVariables|GetLocal%20Attachment) Attachment)
        (bind _returnvalue (Utilities|GetDataTableRow "/Game/UltimateWeaponLoadout/Blueprint/Weapon/DT_Weapons.DT_Weapons" (.Name (Utilities|Struct|BreakS_WeaponConfig (Utilities|Array|Get(acopy) (Variables|Default|GetWeapons) (LocalVariables|Getlocal%20ID)))))
          (:then
            (Utilities|Array|SetArrayElem (Variables|Default|GetWeapons) (LocalVariables|Getlocal%20ID) (Utilities|Struct|MakeS_WeaponConfig (.Name (Utilities|Struct|BreakS_WeaponConfig _returnvalue)) (.Description (Utilities|Struct|BreakS_WeaponConfig _returnvalue)) (.Icon (Utilities|Struct|BreakS_WeaponConfig _returnvalue)) (.Actor (Utilities|Struct|BreakS_WeaponConfig _returnvalue)) (.Socket (Utilities|Struct|BreakS_WeaponConfig _returnvalue)) (.TypeWeapon (Utilities|Struct|BreakS_WeaponConfig _returnvalue)) (.AnimationState (Utilities|Struct|BreakS_WeaponConfig _returnvalue)) (.SkeletalMesh (Utilities|Struct|BreakS_WeaponConfig _returnvalue)) (.ScaleSkeletalmesh (Utilities|Struct|BreakS_WeaponConfig _returnvalue)) (.AttachmentValid (Utilities|Struct|BreakS_WeaponConfig _returnvalue)) (.CameraPositionAttachmentType (Utilities|Struct|BreakS_WeaponConfig _returnvalue)) (LocalVariables|GetLocal%20Attachment) (.StatusWeaponDefault (Utilities|Struct|BreakS_WeaponConfig _returnvalue)) (.StatusWeaponCurrent (Utilities|Struct|BreakS_WeaponConfig _returnvalue)) (.CurrunteLevel (Utilities|Struct|BreakS_WeaponConfig _returnvalue)) (.MaxLevel (Utilities|Struct|BreakS_WeaponConfig _returnvalue)) (.LevelUnlock (Utilities|Struct|BreakS_WeaponConfig _returnvalue)) (.AnimationShowCaseWeapon (Utilities|Struct|BreakS_WeaponConfig _returnvalue)) (.AnimationShowCaseSocketWeaponspawn (Utilities|Struct|BreakS_WeaponConfig _returnvalue))))
            (LocalVariables|SetLocal%20New%20Weapon (Utilities|Struct|MakeS_WeaponConfig (.Name (Utilities|Struct|BreakS_WeaponConfig _returnvalue)) (.Description (Utilities|Struct|BreakS_WeaponConfig _returnvalue)) (.Icon (Utilities|Struct|BreakS_WeaponConfig _returnvalue)) (.Actor (Utilities|Struct|BreakS_WeaponConfig _returnvalue)) (.Socket (Utilities|Struct|BreakS_WeaponConfig _returnvalue)) (.TypeWeapon (Utilities|Struct|BreakS_WeaponConfig _returnvalue)) (.AnimationState (Utilities|Struct|BreakS_WeaponConfig _returnvalue)) (.SkeletalMesh (Utilities|Struct|BreakS_WeaponConfig _returnvalue)) (.ScaleSkeletalmesh (Utilities|Struct|BreakS_WeaponConfig _returnvalue)) (.AttachmentValid (Utilities|Struct|BreakS_WeaponConfig _returnvalue)) (.CameraPositionAttachmentType (Utilities|Struct|BreakS_WeaponConfig _returnvalue)) (LocalVariables|GetLocal%20Attachment) (.StatusWeaponDefault (Utilities|Struct|BreakS_WeaponConfig _returnvalue)) (.StatusWeaponCurrent (Utilities|Struct|BreakS_WeaponConfig _returnvalue)) (.CurrunteLevel (Utilities|Struct|BreakS_WeaponConfig _returnvalue)) (.MaxLevel (Utilities|Struct|BreakS_WeaponConfig _returnvalue)) (.LevelUnlock (Utilities|Struct|BreakS_WeaponConfig _returnvalue)) (.AnimationShowCaseWeapon (Utilities|Struct|BreakS_WeaponConfig _returnvalue)) (.AnimationShowCaseSocketWeaponspawn (Utilities|Struct|BreakS_WeaponConfig _returnvalue))))
            (goto _label Break)))))
    (:Completed
      (return (LocalVariables|GetLocal%20New%20Weapon)))))

(fn GetWeaponSave
  (params (Weapon :type S%20Weapon%20Config%20Structure))
  (for _array_element (Variables|Default|GetWeapons)
    (if (== (.Name (Utilities|Struct|BreakS_WeaponConfig _array_element)) (.Name (Utilities|Struct|BreakS_WeaponConfig Weapon)))
      (return _array_element))))

(fn SaveWeaponSlots
  (params (Weapon :type S%20Weapon%20Config%20Structure) (Slot :type E_TypeSlot%20Enum :default "NewEnumerator2"))
  (switch Utilities|FlowControl|Switch|SwitchonE_TypeSlot Slot
    (:NewEnumerator2
      (Variables|Default|SetWeapon%20Current Weapon))
    (:NewEnumerator0
      (Variables|Default|SetWeapon%20Primary Weapon))
    (:NewEnumerator1
      (Variables|Default|SetWeapon%20Secondary Weapon))))

(fn SaveRemoveAttachmentWeapon
  (params (Weapon :type S%20Weapon%20Config%20Structure) (Attachment :type S%20Attachment%20Type%20Structure))
  (bind (_array_element _array_index) (Utilities|Array|ForEachLoopwithBreak (Variables|Default|GetWeapons) :!label _label)
    (:LoopBody
      (if (== (.Name (Utilities|Struct|BreakS_WeaponConfig _array_element)) (.Name (Utilities|Struct|BreakS_WeaponConfig Weapon)))
        (LocalVariables|Setlocal%20ID _array_index)
        (LocalVariables|SetLocal%20Attachment (.AttachmentCurrent (Utilities|Struct|BreakS_WeaponConfig (Utilities|Array|Get(acopy) (Variables|Default|GetWeapons) (LocalVariables|Getlocal%20ID)))))
        (goto _label Break)))
    (:Completed
      (bind (_array_element_2 _array_index_2) (Utilities|Array|ForEachLoopwithBreak (LocalVariables|GetLocal%20Attachment) :!label _label_2)
        (:LoopBody
          (if (Utilities|Enum|Equal(Enum) (.Name (Utilities|Struct|BreakS_AttachmentType _array_element_2)) (.Name (Utilities|Struct|BreakS_AttachmentType Attachment)))
            (LocalVariables|Setlocal%20Attachment%20Remove%20ID _array_index_2)
            (goto _label_2 Break)))
        (:Completed
          (Utilities|Array|RemoveIndex (LocalVariables|GetLocal%20Attachment) (LocalVariables|Getlocal%20Attachment%20Remove%20ID))
          (bind _returnvalue (Utilities|GetDataTableRow "/Game/UltimateWeaponLoadout/Blueprint/Weapon/DT_Weapons.DT_Weapons" (.Name (Utilities|Struct|BreakS_WeaponConfig (Utilities|Array|Get(acopy) (Variables|Default|GetWeapons) (LocalVariables|Getlocal%20ID)))))
            (:then
              (Utilities|Array|SetArrayElem (Variables|Default|GetWeapons) (LocalVariables|Getlocal%20ID) (Utilities|Struct|MakeS_WeaponConfig (.Name (Utilities|Struct|BreakS_WeaponConfig _returnvalue)) (.Description (Utilities|Struct|BreakS_WeaponConfig _returnvalue)) (.Icon (Utilities|Struct|BreakS_WeaponConfig _returnvalue)) (.Actor (Utilities|Struct|BreakS_WeaponConfig _returnvalue)) (.Socket (Utilities|Struct|BreakS_WeaponConfig _returnvalue)) (.TypeWeapon (Utilities|Struct|BreakS_WeaponConfig _returnvalue)) (.AnimationState (Utilities|Struct|BreakS_WeaponConfig _returnvalue)) (.SkeletalMesh (Utilities|Struct|BreakS_WeaponConfig _returnvalue)) (.ScaleSkeletalmesh (Utilities|Struct|BreakS_WeaponConfig _returnvalue)) (.AttachmentValid (Utilities|Struct|BreakS_WeaponConfig _returnvalue)) (.CameraPositionAttachmentType (Utilities|Struct|BreakS_WeaponConfig _returnvalue)) (LocalVariables|GetLocal%20Attachment) (.StatusWeaponDefault (Utilities|Struct|BreakS_WeaponConfig _returnvalue)) (.StatusWeaponCurrent (Utilities|Struct|BreakS_WeaponConfig _returnvalue)) (.CurrunteLevel (Utilities|Struct|BreakS_WeaponConfig _returnvalue)) (.MaxLevel (Utilities|Struct|BreakS_WeaponConfig _returnvalue)) (.LevelUnlock (Utilities|Struct|BreakS_WeaponConfig _returnvalue)) (.AnimationShowCaseWeapon (Utilities|Struct|BreakS_WeaponConfig _returnvalue)) (.AnimationShowCaseSocketWeaponspawn (Utilities|Struct|BreakS_WeaponConfig _returnvalue))))
              (return (Utilities|Struct|MakeS_WeaponConfig (.Name (Utilities|Struct|BreakS_WeaponConfig _returnvalue)) (.Description (Utilities|Struct|BreakS_WeaponConfig _returnvalue)) (.Icon (Utilities|Struct|BreakS_WeaponConfig _returnvalue)) (.Actor (Utilities|Struct|BreakS_WeaponConfig _returnvalue)) (.Socket (Utilities|Struct|BreakS_WeaponConfig _returnvalue)) (.TypeWeapon (Utilities|Struct|BreakS_WeaponConfig _returnvalue)) (.AnimationState (Utilities|Struct|BreakS_WeaponConfig _returnvalue)) (.SkeletalMesh (Utilities|Struct|BreakS_WeaponConfig _returnvalue)) (.ScaleSkeletalmesh (Utilities|Struct|BreakS_WeaponConfig _returnvalue)) (.AttachmentValid (Utilities|Struct|BreakS_WeaponConfig _returnvalue)) (.CameraPositionAttachmentType (Utilities|Struct|BreakS_WeaponConfig _returnvalue)) (LocalVariables|GetLocal%20Attachment) (.StatusWeaponDefault (Utilities|Struct|BreakS_WeaponConfig _returnvalue)) (.StatusWeaponCurrent (Utilities|Struct|BreakS_WeaponConfig _returnvalue)) (.CurrunteLevel (Utilities|Struct|BreakS_WeaponConfig _returnvalue)) (.MaxLevel (Utilities|Struct|BreakS_WeaponConfig _returnvalue)) (.LevelUnlock (Utilities|Struct|BreakS_WeaponConfig _returnvalue)) (.AnimationShowCaseWeapon (Utilities|Struct|BreakS_WeaponConfig _returnvalue)) (.AnimationShowCaseSocketWeaponspawn (Utilities|Struct|BreakS_WeaponConfig _returnvalue)))))))))))

(fn CheckSaveSlotWeaapon
  (params (Weapon :type S%20Weapon%20Config%20Structure))
  (if (== (.Name (Utilities|Struct|BreakS_WeaponConfig Weapon)) (.Name (Utilities|Struct|BreakS_WeaponConfig (Variables|Default|GetWeapon%20Current))))
    (CallFunction|SaveWeaponSlots Weapon "NewEnumerator2")
    (elif (== (.Name (Utilities|Struct|BreakS_WeaponConfig Weapon)) (.Name (Utilities|Struct|BreakS_WeaponConfig (Variables|Default|GetWeapon%20Primary))))
      (CallFunction|SaveWeaponSlots Weapon "NewEnumerator0")
      (elif (== (.Name (Utilities|Struct|BreakS_WeaponConfig Weapon)) (.Name (Utilities|Struct|BreakS_WeaponConfig (Variables|Default|GetWeapon%20Secondary))))
        (CallFunction|SaveWeaponSlots Weapon "NewEnumerator1")))))