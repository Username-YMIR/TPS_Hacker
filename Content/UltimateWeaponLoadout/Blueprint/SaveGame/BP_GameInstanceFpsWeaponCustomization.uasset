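; Game instance that owns the persistent save data for FPS weapon customization and loadouts.
; On Init it loads the BP_SaveFpsWeaponCustomization slot, or creates one with default weapon data via CreateSaveWeapon and saves it.
; Attachment apply and remove calls delegate to the save object, recheck slot weapons, write to disk and return the result.
; SaveWeaponSlot only forwards to the save object, with no disk write here.
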(event Custom|Save%20Weapon%20Slot
  (params (Weapon :type S%20Weapon%20Config%20Structure) (Type%20Slot%20Weapon :type E_TypeSlot%20Enum :default "NewEnumerator2"))
  (Default|SaveWeaponSlots (Variables|Default|GetCurrentSaveGame) Weapon Type%20Slot%20Weapon))

(event EventInit
  (bind _returnvalue (SaveGame|DoesSaveGameExist (Variables|Default|GetSlot%20Name)))
  (if _returnvalue
    (bind _returnvalue_2 (SaveGame|LoadGamefromSlot (Variables|Default|GetSlot%20Name)))
    (bind _asbp_save_fps_weapon_customization (Utilities|Casting|CastToBP_SaveFpsWeaponCustomization _returnvalue_2))
    (Variables|Default|SetCurrentSaveGame _asbp_save_fps_weapon_customization)
    (else
      (bind _returnvalue_3 (SaveGame|CreateSaveGameObject "/Game/UltimateWeaponLoadout/Blueprint/SaveGame/BP_SaveFpsWeaponCustomization.BP_SaveFpsWeaponCustomization_C"))
      (bind _output_get (Variables|Default|SetCurrentSaveGame _returnvalue_3))
      (Default|CreateSaveWeapon _output_get)
      (SaveGame|SaveGametoSlot (Variables|Default|GetCurrentSaveGame) (Variables|Default|GetSlot%20Name)))))

(fn SaveApplyAttachmentWeapon
  (params (Weapon :type S%20Weapon%20Config%20Structure) (Attachment :type S%20Attachment%20Type%20Structure))
  (bind _currentsavegame (Variables|Default|GetCurrentSaveGame))
  (bind _weapon_new (Default|SaveApplyAttachmentWeapon _currentsavegame Weapon Attachment))
  (Default|CheckSaveSlotWeaapon _currentsavegame _weapon_new)
  (SaveGame|SaveGametoSlot (Variables|Default|GetCurrentSaveGame) (Variables|Default|GetSlot%20Name))
  (return _weapon_new))

(fn SaveRemoveAttachmentWeapon
  (params (Weapon :type S%20Weapon%20Config%20Structure) (Attachment :type S%20Attachment%20Type%20Structure))
  (bind _currentsavegame (Variables|Default|GetCurrentSaveGame))
  (bind _weapon_new (Default|SaveRemoveAttachmentWeapon _currentsavegame Weapon Attachment))
  (Default|CheckSaveSlotWeaapon _currentsavegame _weapon_new)
  (SaveGame|SaveGametoSlot (Variables|Default|GetCurrentSaveGame) (Variables|Default|GetSlot%20Name))
  (return _weapon_new))