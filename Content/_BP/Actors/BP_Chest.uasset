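; BP_Chest is an interactable chest actor whose interaction is currently only a debug placeholder.
; It supplies interaction hooks: CanInteract always allows the interactor, GetInteractText returns the "Chest" label, and GetInteractRoot returns the variable NewVar.
; OnInteract prints a success message containing that label to confirm the call, with no opening or loot logic.
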(event EventBeginPlay)

(event Collision|EventActorBeginOverlap
  (params (OtherActor :type Actor%20Object%20Reference)))

(event EventTick
  (params (DeltaSeconds :type Float%20%28single-precision%29)))

(event EventOnInteract
  (params (Interactor :type Actor%20Object%20Reference))
  (Development|PrintString (Utilities|String|Append "Interact Succeed : " (Utilities|String|ToString(Text) (CallFunction|GetInteractText))) true true "(R=0.000000,G=0.660000,B=1.000000,A=1.000000)" 5.0))

(fn ConstructionScript)

(fn CanInteract
  (params (Interactor :type Actor%20Object%20Reference))
  (return true))

(fn GetInteractRoot
  (return (Variables|Default|GetNewVar)))

(fn GetInteractText
  (return "Chest"))