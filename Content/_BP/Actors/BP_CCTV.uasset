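; BP_CCTV is a security camera actor that acts as a hackable target.
; It supplies hack query functions with placeholder values: it always allows hacking, costs nothing, reports zero range and no root, and labels itself CCTV.
; ExecuteHack only prints a success message with that label, so the camera has no real hacked behavior yet.
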(event EventBeginPlay)

(event Collision|EventActorBeginOverlap
  (params (OtherActor :type Actor%20Object%20Reference)))

(event EventTick
  (params (DeltaSeconds :type Float%20%28single-precision%29)))

(event EventExecuteHack
  (params (Hacker :type Actor%20Object%20Reference))
  (Development|PrintString (Utilities|String|Append "Hacking Succeed : " (Utilities|String|ToString(Text) (CallFunction|GetHackText))) true true "(R=0.000000,G=0.660000,B=1.000000,A=1.000000)" 5.0))

(fn ConstructionScript)

(fn CanHack
  (params (Hacker :type Actor%20Object%20Reference))
  (return true))

(fn GetHackCost
  (return 0))

(fn GetHackRange
  (return 0.0))

(fn GetHackRoot
  (return 0))

(fn GetHackText
  (return "CCTV"))